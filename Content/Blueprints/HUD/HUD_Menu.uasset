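; Main menu HUD that shows the menu widget and lets the player start the game or quit.
; On BeginPlay it creates UW_MainMenu, binds its Play and Quit button clicks to local events, and switches to UI-only input with a visible cursor.
; Play opens the Game level by object reference, and Quit exits the application.
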(event Custom|Quit
  (Game|QuitGame 0 "Quit" false))

(event Custom|Play
  (Game|OpenLevel(byObjectReference) "/Game/Levels/Game.Game"))

(event EventBeginPlay
  (bind _returnvalue (Game|GetPlayerController 0))
  (bind _returnvalue_2 (UserInterface|CreateWidget "/Game/Blueprints/UI/MainMenu/UW_MainMenu.UW_MainMenu_C"))
  (EventDispatchers|BindEventtoOnClicked (Variables|/Game/Blueprints/UI/MainMenu/UW_MainMenu.UW_MainMenu_C|GetPlay _returnvalue_2) (delegate Custom|Play))
  (EventDispatchers|BindEventtoOnClicked (Variables|/Game/Blueprints/UI/MainMenu/UW_MainMenu.UW_MainMenu_C|GetQuit _returnvalue_2) (delegate Custom|Quit))
  (UserInterface|Viewport|AddtoViewport _returnvalue_2 0)
  (Input|SetInputModeUIOnly _returnvalue 0 "DoNotLock" false)
  (Variables|/Script/Engine.PlayerController|SetbShowMouseCursor _returnvalue true))

(fn ConstructionScript)