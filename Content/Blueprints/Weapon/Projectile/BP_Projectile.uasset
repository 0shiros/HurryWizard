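; Projectile fired to place one of the player's two portals, G or D, on surfaces that allow it.
; On hit, it asks actors implementing BPI_Construction whether a portal can be created there, then destroys itself.
; An approved hit teleports the selected existing portal to the impact point, offset and oriented along the normal.
; The moved portal records its hit surface, then it and its linked portal refresh their materials and textures.
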(event OnComponentHit(Sphere)
  (params (HitComponent :type Primitive%20Component%20Object%20Reference) (OtherActor :type Actor%20Object%20Reference) (OtherComp :type Primitive%20Component%20Object%20Reference) (NormalImpulse :type Vector :default "0, 0, 0") (Hit :type Hit%20Result%20Structure%20%28by%20ref%29))
  (bind _player (Variables|Default|GetPlayer))
  (Variables|Default|SetHit Hit)
  (if (Utilities|DoesObjectImplementInterface OtherActor "/Game/Blueprints/Environnement/Surface/Interface/BPI_Construction.BPI_Construction_C")
    (bind _return (Class|BPIConstruction|CanCreatePortal(Message) OtherActor))
    (if _return
      (switch Utilities|FlowControl|Switch|SwitchonE_PortalType (Variables|Default|GetPortalToCreate)
        (:NewEnumerator0
          (CallFunction|TeleportPortal (Variables|/Game/Blueprints/Character/BP_Player.BP_Player_C|GetPortalG _player)))
        (:NewEnumerator1
          (CallFunction|TeleportPortal (Variables|/Game/Blueprints/Character/BP_Player.BP_Player_C|GetPortalD _player))))
      (Actor|DestroyActor)
      (else
        (Actor|DestroyActor)))
    (else
      (Actor|DestroyActor))))

(fn ConstructionScript)

(fn SetLocationandRotation
  (params (HitPoint :type Vector) (HitNormal :type Vector%20%28by%20ref%29))
  (return (+ HitPoint HitNormal) (Math|Rotator|MakeRotfromX HitNormal)))

(fn TeleportPortal
  (params (Portal :type BP%20Portal%20Object%20Reference%20%28by%20ref%29))
  (bind _hit (Variables|Default|GetHit))
  (bind (_returnvalue _returnvalue2) (CallFunction|SetLocationandRotation (.impactpoint _hit) (.normal _hit)))
  (Utilities|IsValid Portal
    (:Is%20Valid
      (Transformation|SetActorLocationAndRotation Portal _returnvalue _returnvalue2 false true)
      (Variables|/Game/Blueprints/PortalSystem/BP_Portal.BP_Portal_C|SetHitSurface Portal (.hitactor _hit))
      (Default|SetMaterialandTexture Portal)
      (Default|SetMaterialandTexture (Variables|/Game/Blueprints/PortalSystem/BP_Portal.BP_Portal_C|GetLinkedPortal Portal)))))