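; BP_TestPortal is a test portal actor that teleports overlapping actors to the location of its linked portal.
; Each tick it allows teleporting only when the rounded Y of ForwardPortal's forward vector opposes that of player 0, a coarse single-axis facing check.
; On Portal overlap, any actor is moved to the linked Portal component, taking the player mesh's world rotation.
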(event OnComponentBeginOverlap(Portal)
  (params (OverlappedComponent :type Primitive%20Component%20Object%20Reference) (OtherActor :type Actor%20Object%20Reference) (OtherComp :type Primitive%20Component%20Object%20Reference) (OtherBodyIndex :type Integer) (bFromSweep :type Boolean) (SweepResult :type Hit%20Result%20Structure%20%28by%20ref%29))
  (if (Variables|Default|GetCanTeleport)
    (Transformation|Teleport OtherActor (Transformation|GetWorldLocation (Variables|BP_TestPortal_C|GetPortal (Variables|Default|GetLinkedPortal))) (Transformation|GetWorldRotation (Variables|/Script/Engine.Character|GetMesh (Game|GetPlayerCharacter 0))))))

(event EventTick
  (params (DeltaSeconds :type Float%20%28single-precision%29))
  (if (== (Math|Float|Round (.y (Math|Vector|GetForwardVector (Variables|Default|GetForwardPortal)))) (* (Math|Float|Round (.y (Transformation|GetActorForwardVector (Game|GetPlayerCharacter 0)))) -1))
    (Variables|Default|SetCanTeleport true)
    (else
      (Variables|Default|SetCanTeleport false))))

(fn ConstructionScript)