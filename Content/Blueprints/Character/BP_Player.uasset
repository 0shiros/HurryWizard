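; Player Blueprint whose SmoothOrientation event eases the player back upright when the controller or capsule has non-zero roll.
; It captures both starting rotations, then plays the Rotate timeline to drive ease-in-out interpolation on each update.
; The control rotation loses its roll while keeping pitch and yaw, and the capsule's world rotation eases to zero on all axes.
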(event Custom|SmoothOrientation
  (params (?ewControlRotation :type Rotator))
  (if (or (!= (.roll (Pawn|GetControlRotation (Game|GetPlayerController 0) :!class /Script/Engine.Controller)) 0.0) (!= (.roll (Transformation|GetWorldRotation (Variables|Collision|GetCapsuleComponent))) 0.0))
    (Variables|Default|SetInitialControlRotation (Pawn|GetControlRotation (Game|GetPlayerController 0) :!class /Script/Engine.Controller))
    (Variables|Default|SetInitialWorldRotation (Transformation|GetWorldRotation (Variables|Collision|GetCapsuleComponent)))
    (bind _alpha (Timeline|Rotate PlayFromStart)
      (:Update
        (Pawn|SetControlRotation (Game|GetPlayerController 0) (Math|Interpolation|Ease "EaseInOut" _alpha (Variables|Default|GetInitialControlRotation) (Math|Rotator|MakeRotator 0.0 (.Pitch (Math|Rotator|BreakRotator (Variables|Default|GetInitialControlRotation))) (.Yaw (Math|Rotator|BreakRotator (Variables|Default|GetInitialControlRotation)))) true))
        (Transformation|SetWorldRotation (Variables|Collision|GetCapsuleComponent) (Math|Interpolation|Ease "EaseInOut" _alpha (Variables|Default|GetInitialWorldRotation) (Math|Rotator|MakeRotator 0.0 0.0 0.0) true) false false)))))

(fn ConstructionScript)