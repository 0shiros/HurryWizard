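; Player controller for a first-person portal game, turning Enhanced Input actions into actions on the possessed BP_Player.
; On start it adds the player mapping context, caches the character and sets game-only input.
; It routes move, look and jump to the character, and left/right shoot fire two portal projectile types.
; Interaction line-traces from the camera to pick up a physics object onto the attach point, or drops it with physics restored.
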(event Custom|Start
  (Input|AddMappingContext (PlayerController|LocalPlayerSubsystems|GetEnhancedInputLocalPlayerSubsystem) "/Game/Input/IMC/IMC_Player.IMC_Player" 0 "(bIgnoreAllPressedKeysUntilRelease=True,bForceImmediately=False,bNotifyUserSettings=False)")
  (bind _asbp_player (Utilities|Casting|CastToBP_Player (Game|GetPlayerCharacter 0)))
  (Variables|Default|SetAs%20BP%20Player _asbp_player)
  (Input|SetInputModeGameOnly self false))

(event Input|EnhancedActionEvents|EnhancedInputActionIAC_Move
  (params (ActionValue :type Vector%202D%20Structure) (ElapsedSeconds :type Float%20%28double-precision%29) (TriggeredSeconds :type Float%20%28double-precision%29) (InputAction :type Input%20Action%20Object%20Reference :default "/Game/Input/IAC/IAC_Move.IAC_Move"))
  (CallFunction|Move (.x ActionValue) (.y ActionValue)))

(event Input|EnhancedActionEvents|EnhancedInputActionIAC_MouseLook
  (params (ActionValue :type Vector%202D%20Structure) (ElapsedSeconds :type Float%20%28double-precision%29) (TriggeredSeconds :type Float%20%28double-precision%29) (InputAction :type Input%20Action%20Object%20Reference :default "/Game/Input/IAC/IAC_MouseLook.IAC_MouseLook"))
  (CallFunction|Aim (.x ActionValue) (.y ActionValue)))

(event Input|EnhancedActionEvents|EnhancedInputActionIAC_Jump
  (params (ActionValue :type Boolean) (ElapsedSeconds :type Float%20%28double-precision%29) (TriggeredSeconds :type Float%20%28double-precision%29) (InputAction :type Input%20Action%20Object%20Reference :default "/Game/Input/IAC/IAC_Jump.IAC_Jump"))
  (bind _as_bp_player (Variables|Default|GetAs%20BP%20Player))
  (:Started
    (Character|Jump _as_bp_player))
  (:Completed
    (Character|StopJumping _as_bp_player)))

(event Input|EnhancedActionEvents|EnhancedInputActionIAC_LeftShoot
  (params (ActionValue :type Boolean) (ElapsedSeconds :type Float%20%28double-precision%29) (TriggeredSeconds :type Float%20%28double-precision%29) (InputAction :type Input%20Action%20Object%20Reference :default "/Game/Input/IAC/IAC_LeftShoot.IAC_LeftShoot"))
  (:Started
    (Default|Shoot (Variables|Default|GetAs%20BP%20Player) (Variables|Default|GetPortalProjectile1))))

(event Input|EnhancedActionEvents|EnhancedInputActionIAC_RightShoot
  (params (ActionValue :type Boolean) (ElapsedSeconds :type Float%20%28double-precision%29) (TriggeredSeconds :type Float%20%28double-precision%29) (InputAction :type Input%20Action%20Object%20Reference :default "/Game/Input/IAC/IAC_RightShoot.IAC_RightShoot"))
  (:Started
    (Default|Shoot (Variables|Default|GetAs%20BP%20Player) (Variables|Default|GetPortalProjectile2))))

(event Input|EnhancedActionEvents|EnhancedInputActionIAC_Interaction
  (params (ActionValue :type Boolean) (ElapsedSeconds :type Float%20%28double-precision%29) (TriggeredSeconds :type Float%20%28double-precision%29) (InputAction :type Input%20Action%20Object%20Reference :default "/Game/Input/IAC/IAC_Interaction.IAC_Interaction"))
  (bind _as_bp_player (Variables|Default|GetAs%20BP%20Player))
  (bind _camera (Variables|/Game/Blueprints/Character/BP_Player.BP_Player_C|GetCamera _as_bp_player))
  (bind _returnvalue (Transformation|GetWorldLocation _camera))
  (:Started
    (if (Variables|/Game/Blueprints/Character/BP_Player.BP_Player_C|GetIsGrabbingObject (Variables|Default|GetAs%20BP%20Player))
      (Transformation|DetachFromActor (Variables|Default|GetHit%20Actor) "KeepWorld" "KeepWorld" "KeepWorld")
      (Physics|SetSimulatePhysics (Variables|Default|GetHit%20Component) true)
      (Variables|/Game/Blueprints/Character/BP_Player.BP_Player_C|SetIsGrabbingObject (Variables|Default|GetAs%20BP%20Player) false)
      (Variables|Default|SetisBeingCarry (Variables|Default|GetHit%20Actor) false)
      (else
        (bind (_outhit _returnvalue_2) (Collision|LineTraceByChannel _returnvalue (+ _returnvalue (* (Math|Vector|GetForwardVector (Transformation|GetWorldRotation _camera)) 2.5e+02)) "TraceTypeQuery1" false 0 "ForDuration"))
        (if _returnvalue_2
          (if (.bSuccess (Utilities|Casting|CastTo (.HitActor (Collision|BreakHitResult _outhit))))
            (Variables|Default|SetHit%20Actor (.AsBP%20Movable (Utilities|Casting|CastTo (.HitActor (Collision|BreakHitResult _outhit)))))
            (Physics|SetSimulatePhysics (.HitComponent (Collision|BreakHitResult _outhit)) false)
            (bind _returnvalue_3 (Transformation|AttachComponentToComponent (.HitActor (Collision|BreakHitResult _outhit)) (Variables|/Game/Blueprints/Character/BP_Player.BP_Player_C|GetAttachPoint (Variables|Default|GetAs%20BP%20Player)) "None" "KeepWorld" "KeepWorld" "KeepWorld" true))
            (Variables|/Game/Blueprints/Character/BP_Player.BP_Player_C|SetIsGrabbingObject (Variables|Default|GetAs%20BP%20Player) _returnvalue_3)
            (Variables|Default|SetHit%20Component (.HitComponent (Collision|BreakHitResult _outhit)))
            (Variables|Default|SetisBeingCarry (Variables|Default|GetHit%20Actor) true)))))))

(fn ConstructionScript)

(fn Move
  (params (Left/Right :type Float%20%28double-precision%29) (Forward/Backward :type Float%20%28double-precision%29))
  (bind _as_bp_player (Variables|Default|GetAs%20BP%20Player))
  (Pawn|Input|AddMovementInput _as_bp_player (Transformation|GetActorRightVector _as_bp_player) Left/Right false)
  (Pawn|Input|AddMovementInput _as_bp_player (Transformation|GetActorForwardVector _as_bp_player) Forward/Backward false))

(fn Aim
  (params (Yaw :type Float%20%28single-precision%29) (Pitch :type Float%20%28single-precision%29))
  (bind _as_bp_player (Variables|Default|GetAs%20BP%20Player))
  (Pawn|Input|AddControllerYawInput _as_bp_player Yaw)
  (Pawn|Input|AddControllerPitchInput _as_bp_player Pitch))

(fn Jump)