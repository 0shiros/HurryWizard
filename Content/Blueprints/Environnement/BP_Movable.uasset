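; Movable prop that interacts with linked BP_Portals using two components, Real and Copy.
; Real's overlaps set or clear the current portal, and each Tick a dot product against the portal's forward direction tests the actor's side.
; Past that threshold, a carried prop shows Copy at the linked portal with its location rotated 180 degrees, while an uncarried one teleports Real via UpdateLocation.
; Otherwise Copy snaps back onto Real.
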(event OnComponentBeginOverlap(Real)
  (params (OverlappedComponent :type Primitive%20Component%20Object%20Reference) (OtherActor :type Actor%20Object%20Reference) (OtherComp :type Primitive%20Component%20Object%20Reference) (OtherBodyIndex :type Integer) (bFromSweep :type Boolean) (SweepResult :type Hit%20Result%20Structure%20%28by%20ref%29))
  (bind (_asbp_portal _bsuccess) (Utilities|Casting|CastToBP_Portal OtherActor))
  (if _bsuccess
    (Variables|Default|SetAs%20BP%20Portal _asbp_portal)))

(event OnComponentEndOverlap(Real)
  (params (OverlappedComponent :type Primitive%20Component%20Object%20Reference) (OtherActor :type Actor%20Object%20Reference) (OtherComp :type Primitive%20Component%20Object%20Reference) (OtherBodyIndex :type Integer))
  (Variables|Default|SetAs%20BP%20Portal 0)
  (Transformation|DetachFromComponent (Variables|Default|GetCopy) "KeepWorld" "KeepWorld" "KeepWorld" true)
  (Transformation|AttachComponentToComponent (Variables|Default|GetCopy) (Variables|Default|GetReal) "None" "KeepWorld" "KeepWorld" "KeepWorld" true)
  (Transformation|SetRelativeTransform (Variables|Default|GetCopy) (Math|Transform|MakeTransform "0, 0, 0" "0, 0, 0" "1.000000,1.000000,1.000000") false true))

(event EventTick
  (params (DeltaSeconds :type Float%20%28single-precision%29))
  (bind _real (Variables|Default|GetReal))
  (bind _as_bp_portal (Variables|Default|GetAs%20BP%20Portal))
  (bind _as_bp_portal_2 (Variables|Default|GetAs%20BP%20Portal))
  (bind _returnvalue (Transformation|GetWorldTransform _real))
  (bind _portalplane (Variables|/Game/Blueprints/PortalSystem/BP_Portal.BP_Portal_C|GetPortalPlane _as_bp_portal))
  (bind _returnvalue_2 (Transformation|GetWorldTransform _portalplane))
  (bind _returnvalue_3 (Math|Transform|MakeRelativeTransform _returnvalue _returnvalue_2))
  (Utilities|IsValid (Variables|Default|GetAs%20BP%20Portal)
    (:Is%20Valid
      (if (< (Math|Vector|DotProduct (Math|Vector|Normalize (- (Transformation|GetActorLocation) (Transformation|GetActorLocation _as_bp_portal_2))) (Math|Vector|GetForwardVector (Variables|/Game/Blueprints/PortalSystem/BP_Portal.BP_Portal_C|GetForwardDirection _as_bp_portal_2))) 0.5)
        (if (Variables|Default|GetisBeingCarry)
          (Transformation|DetachFromComponent (Variables|Default|GetCopy) "KeepWorld" "KeepWorld" "KeepWorld" true)
          (Transformation|AttachComponentToComponent (Variables|Default|GetCopy) (Variables|/Game/Blueprints/PortalSystem/BP_Portal.BP_Portal_C|GetPortalPlane (Variables|/Game/Blueprints/PortalSystem/BP_Portal.BP_Portal_C|GetLinkedPortal (Variables|Default|GetAs%20BP%20Portal))) "None" "KeepWorld" "KeepWorld" "KeepWorld" true)
          (Transformation|SetRelativeTransform (Variables|Default|GetCopy) (Math|Transform|MakeTransform (Math|Vector|RotateVectorAroundAxis (.location _returnvalue_3) 1.8e+02 (Math|Vector|GetUpVector _portalplane)) (.rotation _returnvalue_3) (.scale _returnvalue_3)) false true)
          (else
            (Transformation|SetWorldTransform (Variables|Default|GetReal) (Math|Transform|MakeTransform (Default|UpdateLocation (Variables|Default|GetAs%20BP%20Portal) (Transformation|GetWorldLocation (Variables|Default|GetCopy))) "0, 0, 0" "1.000000,1.000000,1.000000") false true)
            (Development|PrintString "Hello")))
        (else
          (Transformation|DetachFromComponent (Variables|Default|GetCopy) "KeepWorld" "KeepWorld" "KeepWorld" true)
          (Transformation|AttachComponentToComponent (Variables|Default|GetCopy) (Variables|Default|GetReal) "None" "KeepWorld" "KeepWorld" "KeepWorld" true)
          (Transformation|SetRelativeTransform (Variables|Default|GetCopy) (Math|Transform|MakeTransform "0, 0, 0" "0, 0, 0" "1.000000,1.000000,1.000000") false true))))))

(fn ConstructionScript
  (|CallParentFunction))